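; BP_Arrow is an arrow projectile actor tied to the third-person main character.
; The fire event adds a projectile movement component at runtime and launches it along the given direction at fixed speed.
; The Munich event decrements the player's ammo count through a DoOnce and writes it as text to what appears to be a UI variable.
; Hit is empty, and zombie damage and animation logic is left unconnected.
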(event `Munich`
  ;[1 1 1] actual_(a)
  (bind _asbp_third_personmain (cast `/Game/Main_Character/personaje/BP_ThirdPersonmain` (`GameplayStatics.GetPlayerCharacter` 0)))
  (`/Engine/EditorBlueprintResources/StandardMacros.DoOnce` false
    (:`Completed`
      (bind _output_get (set `/Game/Main_Character/personaje/BP_ThirdPersonmain.Municicon` (- (`/Game/Main_Character/personaje/BP_ThirdPersonmain.Municicon` _asbp_third_personmain) 1) _asbp_third_personmain))
      (set `/Game/Hud_y_UI/UI.Municion` (`KismetStringLibrary.Conv_IntToString` _output_get) (`self.NewVar`)))))

(event `fire`
  (params (direction :type "Vector Structure"))
  ;[1 1 1] actual_(z)
  (bind _returnvalue (`AddComponent|NODE_AddProjectileMovementComponent-0`))
  (set `MovementComponent.Velocity` (* direction 2000.0) _returnvalue))

(event `self.ReceiveHit`
  (params (MyComp :type "PrimitiveComponent Object Reference") (Other :type "Actor Object Reference") (OtherComp :type "PrimitiveComponent Object Reference") (bSelfMoved :type Boolean) (HitLocation :type "Vector Structure") (HitNormal :type "Vector Structure") (NormalImpulse :type "Vector Structure") (Hit :type "HitResult Structure (by ref)")))

(fn `UserConstructionScript`)