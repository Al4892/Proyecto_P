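; BP_SaveGameInstance handles saving and loading of the player's level and position through a BP_Guardar save object.
; SavedGame writes the player character's transform and current level name to a save slot.
; MenuLoadGame sets a load flag, reads the slot through GameLoad, opens the saved level and switches input to game-only.
; A separate LoadGame function applies the stored transform to the player character.
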(event `MenuLoadGame`
  (bind _returnvalue (`GameplayStatics.GetPlayerController` 0))
  (set `self.LoadGame?` true)
  (bind _savedlevel (`self.GameLoad`))
  (`GameplayStatics.OpenLevel` (`KismetStringLibrary.Conv_StringToName` _savedlevel))
  (set `PlayerController.bShowMouseCursor` false _returnvalue)
  (`WidgetBlueprintLibrary.SetInputMode_GameOnly` _returnvalue))

(fn `GameLoad`
  (returns (SavedLevel :type String))
  (bind _returnvalue (`GameplayStatics.LoadGameFromSlot` (`self.SlotNameSave`)))
  (bind _asbp_guardar (cast `/Game/Blueprints/SaveGame/BP_Guardar` _returnvalue))
  (bind _output_get (set `self.SaveRef` _asbp_guardar))
  (return (`/Game/Blueprints/SaveGame/BP_Guardar.SavedLevel` _output_get)))

(fn `LoadGame`
  (`Actor.K2_SetActorTransform` (`self.PlayerCharacter`) (`/Game/Blueprints/SaveGame/BP_Guardar.SavePo` (`self.SaveRef`)) false false))

(fn `SavedGame`
  (bind _returnvalue (`GameplayStatics.CreateSaveGameObject` "/Game/Blueprints/SaveGame/BP_Guardar.BP_Guardar_C"))
  (bind _output_get (set `self.SaveRef` _returnvalue))
  (set `/Game/Blueprints/SaveGame/BP_Guardar.SavePo` (`Actor.GetTransform` (`self.PlayerCharacter`)) _output_get)
  (bind _returnvalue_2 (`GameplayStatics.GetCurrentLevelName` true))
  (set `/Game/Blueprints/SaveGame/BP_Guardar.SavedLevel` _returnvalue_2 (`self.SaveRef`))
  (`GameplayStatics.SaveGameToSlot` (`self.SaveRef`) (`self.SlotNameSave`)))