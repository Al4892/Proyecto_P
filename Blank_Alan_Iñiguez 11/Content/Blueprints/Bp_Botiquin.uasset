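; Health pickup (first-aid kit) that restores the third-person player's health on contact.
; When its collider overlaps BP_ThirdPersonmain, it adds a fixed amount to Salud, clamped to the maximum, prints the new value and destroys itself.
; At full health it only prints a message and stays in the world.
; A disconnected older version using a Vida variable remains in the graph but never runs.
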(event `self.Collider.OnComponentBeginOverlap`
  (params (OverlappedComponent :type "PrimitiveComponent Object Reference") (OtherActor :type "Actor Object Reference") (OtherComp :type "PrimitiveComponent Object Reference") (OtherBodyIndex :type Integer) (bFromSweep :type Boolean) (SweepResult :type "HitResult Structure (by ref)"))
  (bind _asbp_third_personmain (cast `/Game/Main_Character/personaje/BP_ThirdPersonmain` OtherActor))
  ;[0.7 0 1] ACTUAL_(Z)
  (if (== (`/Game/Main_Character/personaje/BP_ThirdPersonmain.salud` _asbp_third_personmain) 100.0)
    (`KismetSystemLibrary.PrintString` "MAXIMUM HEALTH REACHED" true true (struct :`R` 0.002067 :`G` 1.0 :`A` 1.0))
    (else
      (bind _output_get (set `/Game/Main_Character/personaje/BP_ThirdPersonmain.salud` (`KismetMathLibrary.FClamp` (+ (`/Game/Main_Character/personaje/BP_ThirdPersonmain.salud` _asbp_third_personmain) 20.0) 0.0 100.0) _asbp_third_personmain))
      (`KismetSystemLibrary.PrintString` (`KismetStringLibrary.Conv_DoubleToString` _output_get))
      (`self.K2_DestroyActor`))))

(fn `UserConstructionScript`)