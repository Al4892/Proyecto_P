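; BP_Daño is a damage actor that drains the Vida of any BP_ThirdPersonmain that overlaps its Box.
; The overlap and Tick share one chain: cast the overlap's OtherActor, wait on a Delay, then subtract Daño and print the result.
; Tick reuses the last overlapped actor, so damage repeats at the Delay interval with no end-overlap check.
; At zero or below, it prints a death message and calls Ragdoll.
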(event `self.ReceiveTick`
  (params (DeltaSeconds :type "Float (single-precision)"))
  (bind _asbp_third_personmain (cast `/Game/prueba/personaje/BP_ThirdPersonmain` (stale `self.Box.OnComponentBeginOverlap` OtherActor) :!label _label))
  (`KismetSystemLibrary.Delay` 2.0)
  (bind _output_get (set `/Game/prueba/personaje/BP_ThirdPersonmain.Vida` (- (`/Game/prueba/personaje/BP_ThirdPersonmain.Vida` _asbp_third_personmain) (`self.Daño`)) _asbp_third_personmain))
  (if (<= _output_get 0.0)
    (`KismetSystemLibrary.PrintString` "moriste wacghin")
    (`/Game/prueba/personaje/BP_ThirdPersonmain.Ragdoll` _asbp_third_personmain)
    (else
      (`KismetSystemLibrary.PrintString` (`KismetStringLibrary.Conv_DoubleToString` _output_get)))))

(event `self.Box.OnComponentBeginOverlap`
  (params (OverlappedComponent :type "PrimitiveComponent Object Reference") (OtherActor :type "Actor Object Reference") (OtherComp :type "PrimitiveComponent Object Reference") (OtherBodyIndex :type Integer) (bFromSweep :type Boolean) (SweepResult :type "HitResult Structure (by ref)"))
  (goto _label))

(fn `UserConstructionScript`)