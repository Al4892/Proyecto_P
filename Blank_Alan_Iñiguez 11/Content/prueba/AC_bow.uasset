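; AC_bow is an actor component that gives its owning Character a bow with aiming and arrow firing.
; On BeginPlay it spawns the bow and attaches it to a left-hand mesh socket.
; Aiming switches the character to controller-facing rotation, updates the bow's state and spawns an arrow on a right-hand socket; ending aim reverts this and destroys the arrow.
; Firing detaches the arrow and launches it along the camera's forward vector.
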(event `self.ReceiveBeginPlay`
  (bind _ascharacter (cast `Character` (`self.GetOwner`)))
  (set `self.Character` _ascharacter)
  (`self.equipar arma`))

(event `start aim`
  (bind _charactermovement (`Character.CharacterMovement` (`self.Character`)))
  (set `self.Is_aiming` true)
  (set `CharacterMovementComponent.bOrientRotationToMovement` false _charactermovement)
  (set `CharacterMovementComponent.bUseControllerDesiredRotation` true _charactermovement)
  (set `/Game/prueba/BP_bow.BowStates` "NewEnumerator1" (`self.BowVar`))
  (`self.Spawn_Arrow`))

(event `end aim`
  (bind _charactermovement (`Character.CharacterMovement` (`self.Character`)))
  (set `self.Is_aiming` false)
  (set `CharacterMovementComponent.bOrientRotationToMovement` true _charactermovement)
  (set `CharacterMovementComponent.bUseControllerDesiredRotation` false _charactermovement)
  (set `/Game/prueba/BP_bow.BowStates` "NewEnumerator0" (`self.BowVar`))
  (`self.Destroy_Arrow`))

(event `FIRE_START_ARROW`
  (bind _arrowvar (`self.ArrowVar`)
    (:`then`
      (`Actor.K2_DetachFromActor` _arrowvar "KeepWorld" "KeepWorld" "KeepWorld")
      (`/Game/prueba/BP_Arrow.fire` _arrowvar (`SceneComponent.GetForwardVector` (`Actor.GetComponentByClass` (`self.Character`) "/Script/Engine.CameraComponent"))))
    (:`else`)))

(fn `Destroy_Arrow`
  (bind _arrowvar (`self.ArrowVar`)
    (:`then`
      (`Actor.K2_DestroyActor` _arrowvar))
    (:`else`)))

(fn `equipar arma`
  (bind _returnvalue (`|SpawnActorFromClass` (`self.bow_class`) (`KismetMathLibrary.MakeTransform` (0.0 0.0 0.0)) "Undefined" "MultiplyWithRoot" null null))
  (bind _output_get (set `self.BowVar` _returnvalue))
  (`Actor.K2_AttachToComponent` _output_get (`Character.Mesh` (`self.Character`)) "bow_LSocket" "SnapToTarget" "SnapToTarget" "SnapToTarget" true))

(fn `Spawn_Arrow`
  (bind _returnvalue (`|SpawnActorFromClass` "/Game/prueba/BP_Arrow.BP_Arrow_C" (`KismetMathLibrary.MakeTransform` (0.0 0.0 0.0)) "Undefined" "MultiplyWithRoot" null null))
  (bind _output_get (set `self.ArrowVar` _returnvalue))
  (`Actor.K2_AttachToComponent` _output_get (`Character.Mesh` (`self.Character`)) "arrow_rSocket" "SnapToTarget" "SnapToTarget" "SnapToTarget" true))